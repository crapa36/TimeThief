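; GM_Test is a test game mode that creates a WBP_Inventory widget on BeginPlay.
; The widget is never displayed, because the nodes that add it to the viewport and initialize it with the player's BP_TimeThiefCharacter are disconnected.
; A Game-and-UI input mode call is also left unwired, and Tick is disabled.
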(event `self.ReceiveBeginPlay`
  (`parent.ReceiveBeginPlay`)
  (bind _returnvalue (`|CreateWidget` "/Game/KHI/UI/Inventory/WBP_Inventory.WBP_Inventory_C")))

(fn `UserConstructionScript`
  (`parent.UserConstructionScript`))