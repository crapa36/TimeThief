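; BP_MorphingTestCharacter is a test character for switching the type of its MorphingMesh by keyboard.
; The 1, 2 and 3 keys call SetType on MorphingMesh with types A, B and C respectively.
; The morphing itself is not implemented in these graphs, and the construction script only calls its parent.
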(event `Key|One`
  (params (Key :type "Key Structure"))
  (:`Pressed`
    (`MorphingMeshComponent.SetType` (`self.MorphingMesh`) "A")))

(event `Key|Two`
  (params (Key :type "Key Structure"))
  (:`Pressed`
    (`MorphingMeshComponent.SetType` (`self.MorphingMesh`) "B")))

(event `Key|Three`
  (params (Key :type "Key Structure"))
  (:`Pressed`
    (`MorphingMeshComponent.SetType` (`self.MorphingMesh`) "C")))

(fn `UserConstructionScript`
  (`parent.UserConstructionScript`))