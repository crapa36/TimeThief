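; BP_DamageActor is a damage zone that hurts a BP_TimeThiefCharacter standing inside its Box.
; Box overlap begin stores the character as TargetActor, and overlap end clears it if that same character leaves.
; Tick applies frame-rate-independent damage to the valid target every frame by scaling a fixed rate with DeltaSeconds.
; Only one target is tracked at a time, so a newly entering character replaces the previous one.
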(event `self.ReceiveTick`
  (params (DeltaSeconds :type "Float (single-precision)"))
  (if (`KismetSystemLibrary.IsValid` (`self.Target Actor`))
    (`GameplayStatics.ApplyDamage` (`self.Target Actor`) (* DeltaSeconds 50.0))))

(event `self.Box.OnComponentBeginOverlap`
  (params (OverlappedComponent :type "PrimitiveComponent Object Reference") (OtherActor :type "Actor Object Reference") (OtherComp :type "PrimitiveComponent Object Reference") (OtherBodyIndex :type Integer) (bFromSweep :type Boolean) (SweepResult :type "HitResult Structure (by ref)"))
  (bind _asbp_time_thief_character (cast `/Game/Game/Player/BP_TimeThiefCharacter` OtherActor))
  (set `self.Target Actor` _asbp_time_thief_character))

(event `self.Box.OnComponentEndOverlap`
  (params (OverlappedComponent :type "PrimitiveComponent Object Reference") (OtherActor :type "Actor Object Reference") (OtherComp :type "PrimitiveComponent Object Reference") (OtherBodyIndex :type Integer))
  (bind _asbp_time_thief_character (cast `/Game/Game/Player/BP_TimeThiefCharacter` OtherActor))
  (if (== _asbp_time_thief_character (`self.Target Actor`))
    (set `self.Target Actor` null)))

(fn `UserConstructionScript`)